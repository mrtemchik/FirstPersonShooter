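; Knife weapon Blueprint for the first-person character, providing a short-range melee attack.
; Fire is gated by a brief cooldown and plays one of three random attack montages on the player's Mesh2P.
; It also runs a short camera trace, offset randomly by BulletSprey, and passes the result to spawn a Bullet_decal.
; Gun-style ammo, gunshot and muzzle flash functions are present, but Fire never calls them.
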(event `self.Fire`
  (bind _mesh2p (`/Game/FirstPersonBP/Blueprints/FirstPersonCharacter.Mesh2P` (cast `/Game/FirstPersonBP/Blueprints/FirstPersonCharacter` (`GameplayStatics.GetPlayerCharacter` 0) :!pure true)))
  (if (not (`self.cooldown`))
    (set `self.cooldown` true)
    (`|ExecutionSequence`
      (:`then_0`
        (switch `int` (`KismetMathLibrary.RandomIntegerInRange` 0 2)
          (:`0`
            (`|PlayMontage` _mesh2p "/Game/8/Arms_Knife_Attack_01_anim_Montage.Arms_Knife_Attack_01_anim_Montage"))
          (:`1`
            (`|PlayMontage` _mesh2p "/Game/8/Arms_Knife_Attack_02_anim_Montage.Arms_Knife_Attack_02_anim_Montage"))
          (:`2`
            (`|PlayMontage` _mesh2p "/Game/8/Arms_Knife_Attack_03_anim_Montage.Arms_Knife_Attack_03_anim_Montage"))))
      (:`then_1`
        (bind (_start_location _impactpoint) (`self.Line_Trace`))
        (`self.spawn_decal_tracer` _impactpoint _impactpoint))
      (:`then_2`
        (`KismetSystemLibrary.RetriggerableDelay` 0.2)
        (set `self.cooldown` false)))))

(fn `Ammo_check`
  (bind _returnvalue (`KismetMathLibrary.RandomFloatInRange` 0.7 1.2))
  (`/Engine/EditorBlueprintResources/StandardMacros.DecrementInt` (`self.Ammo_Count`)
    (:`  `
      (`GameplayStatics.PlaySoundAtLocation` "/Game/4/Gunshot.Gunshot" (`self.K2_GetActorLocation`) (struct) (* _returnvalue 2.5) _returnvalue 0.0 "/Game/4/NewSoundAttenuation.NewSoundAttenuation" "/Game/4/NewSoundConcurrency.NewSoundConcurrency" null)
      (`SkeletalMeshComponent.PlayAnimation` (`self.SkeletalMesh`) "/Game/2/AK_Fire_anim.AK_Fire_anim" false))))

(fn `Line_Trace`
  (returns (`Start location` :type "Vector Structure") (ImpactPoint :type "Vector Structure"))
  (bind _bullet_sprey (`self.Bullet_Sprey`))
  (bind _returnvalue (* _bullet_sprey -1.0))
  (bind _firstpersoncamera (`/Game/FirstPersonBP/Blueprints/FirstPersonCharacter.FirstPersonCamera` (cast `/Game/FirstPersonBP/Blueprints/FirstPersonCharacter` (`GameplayStatics.GetPlayerCharacter` 0) :!pure true)))
  (bind _returnvalue_2 (`SceneComponent.K2_GetComponentLocation` _firstpersoncamera))
  (bind (_outhit _returnvalue_3) (`KismetSystemLibrary.LineTraceSingle` _returnvalue_2 (+ (+ _returnvalue_2 (* (`SceneComponent.GetForwardVector` _firstpersoncamera) 200.0)) (`KismetMathLibrary.MakeVector` (`KismetMathLibrary.RandomFloatInRange` _returnvalue _bullet_sprey) (`KismetMathLibrary.RandomFloatInRange` _returnvalue _bullet_sprey) (`KismetMathLibrary.RandomFloatInRange` _returnvalue _bullet_sprey))) "TraceTypeQuery1"))
  (if _returnvalue_3
    (bind (_bblockinghit _binitialoverlap _time _distance _location _impactpoint _normal _impactnormal) (`GameplayStatics.BreakHitResult` _outhit))
    (return _impactnormal _impactpoint)))

(fn `spawn_decal_tracer`
  (params (`spawn trnsofrm` :type "Vector Structure") (`Impact point` :type "Vector Structure"))
  (bind (_returnvalue_roll _returnvalue_pitch _returnvalue_yaw) (`KismetMathLibrary.BreakRotator` (`KismetMathLibrary.Conv_VectorToRotator` `Impact point`)))
  (bind _firstpersoncamera (`/Game/FirstPersonBP/Blueprints/FirstPersonCharacter.FirstPersonCamera` (cast `/Game/FirstPersonBP/Blueprints/FirstPersonCharacter` (`GameplayStatics.GetPlayerCharacter` 0) :!pure true)))
  (bind _returnvalue_roll_2 (`KismetMathLibrary.BreakRotator` (`SceneComponent.K2_GetComponentRotation` _firstpersoncamera)))
  (bind (_returnvalue_roll_3 _returnvalue_pitch_2 _returnvalue_yaw_2) (`KismetMathLibrary.BreakRotator` (`KismetMathLibrary.Conv_VectorToRotator` (`SceneComponent.GetForwardVector` _firstpersoncamera))))
  (if (== `spawn trnsofrm` (0.0 0.0 1.0))
    (`|SpawnActorFromClass` "/Game/4/Bullet_decal.Bullet_decal_C" (`KismetMathLibrary.MakeTransform` `spawn trnsofrm` (`KismetMathLibrary.MakeRotator` -90.0 90.0 _returnvalue_yaw_2) (0.01 0.01 0.01)) "Undefined" "OverrideRootScale" null null)
    (else
      (`|SpawnActorFromClass` "/Game/4/Bullet_decal.Bullet_decal_C" (`KismetMathLibrary.MakeTransform` (`KismetMathLibrary.MakeVector` (+ _returnvalue_roll_2 90.0) _returnvalue_pitch (+ _returnvalue_yaw 180.0)) (struct) `spawn trnsofrm`) "Undefined" "OverrideRootScale" null null)))
  (return))

(fn `UserConstructionScript`
  (`parent.UserConstructionScript`)
  (set `self.Name` "NewEnumerator0")
  (set `self.Variable_mode` false))