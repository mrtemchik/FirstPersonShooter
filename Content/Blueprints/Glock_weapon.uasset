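; Glock weapon for the first-person character, with fire, reload, scope and an Unequip that saves its state to SecondGlock.
; Fire spends ammo and traces from the camera with random spread, spawning decal, tracer and muzzle flash, without applying damage.
; Reload uses a DoOnce and delay to refill ammo.
; Scope lerps FOV and arms position via timeline, but its hardcoded true branch leaves zoom-out unreachable.
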(event `self.Unequip`
  (set `/Game/FirstPersonBP/Blueprints/FirstPersonCharacter.second_Glock` (make `/Game/Blueprints/gun_data` "Glock_weapon_C" "NewEnumerator3" (`self.Ammo_Count`) (`self.Max_Ammo`) (`self.Reloading_Time`) (`self.Bullet_Sprey`)) (cast `/Game/FirstPersonBP/Blueprints/FirstPersonCharacter` (`GameplayStatics.GetPlayerCharacter` 0) :!pure true)))

(event `self.Fire`
  (bind _asfirst_person_character (cast `/Game/FirstPersonBP/Blueprints/FirstPersonCharacter` (`GameplayStatics.GetPlayerCharacter` 0) :!pure true))
  (bind _mesh2p (`/Game/FirstPersonBP/Blueprints/FirstPersonCharacter.Mesh2P` _asfirst_person_character))
  (if (> (`self.Ammo_Count`) 0)
    (`self.Ammo_check`)
    (bind (_start_location _impactpoint) (`self.Line_Trace`))
    (`self.spawn_decal_tracer` _start_location _impactpoint _impactpoint)
    (if (`/Game/FirstPersonBP/Blueprints/FirstPersonCharacter.Aim_down` _asfirst_person_character)
      (`|PlayMontage` _mesh2p "/Game/6/Arms_Glock_ADS_Fire_anim_Montage.Arms_Glock_ADS_Fire_anim_Montage"
        (:`then`
          _))
      (else
        (`|PlayMontage` _mesh2p "/Game/5/Arms_Glock_Fire_anim_Montage.Arms_Glock_Fire_anim_Montage"
          (:`then`
            _))))
    (`self.Flash`)
    (else
      (`GameplayStatics.SpawnSoundAtLocation` "/Game/4/DryFire.DryFire" (`self.K2_GetActorLocation`) (struct) 1.0 1.0 0.0 "/Game/4/NewSoundAttenuation.NewSoundAttenuation" "/Game/4/NewSoundConcurrency.NewSoundConcurrency"))))

(event `self.Reload`
  (bind _asfirst_person_character (cast `/Game/FirstPersonBP/Blueprints/FirstPersonCharacter` (`GameplayStatics.GetPlayerCharacter` 0) :!pure true))
  (if (< (`self.Ammo_Count`) (`self.Max_Ammo`))
    (`/Engine/EditorBlueprintResources/StandardMacros.DoOnce` false :!label _label
      (:`Completed`
        (set `/Game/FirstPersonBP/Blueprints/FirstPersonCharacter.Is_reload` true _asfirst_person_character)
        (`|PlayMontage` (`/Game/FirstPersonBP/Blueprints/FirstPersonCharacter.Mesh2P` _asfirst_person_character) "/Game/5/Arms_Glock_Reload_anim_Montage.Arms_Glock_Reload_anim_Montage"
          (:`then`
            (`SkeletalMeshComponent.PlayAnimation` (`self.SkeletalMesh`) "/Game/5/Glock_Reload_anim.Glock_Reload_anim" false)
            (`KismetSystemLibrary.Delay` (`self.Reloading_Time`))
            (set `self.Ammo_Count` (`self.Max_Ammo`))
            (set `/Game/FirstPersonBP/Blueprints/FirstPersonCharacter.Is_reload` false (cast `/Game/FirstPersonBP/Blueprints/FirstPersonCharacter` (`GameplayStatics.GetPlayerCharacter` 0) :!pure true))
            (goto _label :!via `Reset`)))))))

(event `self.Scope`
  (params (Tog :type Boolean))
  (bind _asfirst_person_character (cast `/Game/FirstPersonBP/Blueprints/FirstPersonCharacter` (`GameplayStatics.GetPlayerCharacter` 0) :!pure true))
  (bind _firstpersoncamera (`/Game/FirstPersonBP/Blueprints/FirstPersonCharacter.FirstPersonCamera` _asfirst_person_character))
  (bind _mesh2p (`/Game/FirstPersonBP/Blueprints/FirstPersonCharacter.Mesh2P` _asfirst_person_character))
  (if true
    (bind (_direction _newtrack_0) (`Timeline|Timeline_0` :!via `PlayFromStart`)
      (:`Update`
        (`CameraComponent.SetFieldOfView` _firstpersoncamera (`KismetMathLibrary.Lerp` 90.0 45.0 _newtrack_0))
        (`SceneComponent.K2_SetRelativeTransform` _mesh2p (`KismetMathLibrary.MakeTransform` (`KismetMathLibrary.VLerp` (5.898139 -6.467392 -25.529276) (5.898139 0.0 -16.0) _newtrack_0)) false false)))
    (else
      (bind (_direction_2 _newtrack_0_2) (`Timeline|Timeline_1` :!via `PlayFromStart`)
        (:`Update`
          (`CameraComponent.SetFieldOfView` _firstpersoncamera (`KismetMathLibrary.Lerp` 45.0 90.0 _newtrack_0_2))
          (`SceneComponent.K2_SetRelativeTransform` _mesh2p (`KismetMathLibrary.MakeTransform` (`KismetMathLibrary.VLerp` (5.898139 0.0 -16.0) (5.898139 -6.467392 -25.529276) _newtrack_0_2)) false false))))))

(fn `Ammo_check`
  (bind _returnvalue (`KismetMathLibrary.RandomFloatInRange` 0.7 1.2))
  (`/Engine/EditorBlueprintResources/StandardMacros.DecrementInt` (`self.Ammo_Count`)
    (:`  `
      (`GameplayStatics.PlaySoundAtLocation` "/Game/4/Gunshot.Gunshot" (`self.K2_GetActorLocation`) (struct) (* _returnvalue 2.5) _returnvalue 0.0 "/Game/4/NewSoundAttenuation.NewSoundAttenuation" "/Game/4/NewSoundConcurrency.NewSoundConcurrency" null)
      (`SkeletalMeshComponent.PlayAnimation` (`self.SkeletalMesh`) "/Game/5/Glock_Fire_anim.Glock_Fire_anim" false))))

(fn `Line_Trace`
  (returns (`Start location` :type "Vector Structure") (ImpactPoint :type "Vector Structure"))
  (bind _bullet_sprey (`self.Bullet_Sprey`))
  (bind _returnvalue (`SceneComponent.K2_GetComponentLocation` (`self.Scene`)))
  (bind _returnvalue_2 (* _bullet_sprey -1.0))
  (bind _firstpersoncamera (`/Game/FirstPersonBP/Blueprints/FirstPersonCharacter.FirstPersonCamera` (cast `/Game/FirstPersonBP/Blueprints/FirstPersonCharacter` (`GameplayStatics.GetPlayerCharacter` 0) :!pure true)))
  (bind _returnvalue_3 (`SceneComponent.K2_GetComponentLocation` _firstpersoncamera))
  (bind _outhit (`KismetSystemLibrary.LineTraceSingle` _returnvalue_3 (+ (+ _returnvalue_3 (* (`SceneComponent.GetForwardVector` _firstpersoncamera) 20000.0)) (`KismetMathLibrary.MakeVector` (`KismetMathLibrary.RandomFloatInRange` _returnvalue_2 _bullet_sprey) (`KismetMathLibrary.RandomFloatInRange` _returnvalue_2 _bullet_sprey) (`KismetMathLibrary.RandomFloatInRange` _returnvalue_2 _bullet_sprey))) "TraceTypeQuery1"))
  (bind (_bblockinghit _binitialoverlap _time _distance _location _impactpoint) (`GameplayStatics.BreakHitResult` _outhit))
  (`KismetSystemLibrary.LineTraceSingle` :`Start` _returnvalue :`End` _impactpoint :`TraceChannel` "TraceTypeQuery1" :`TraceColor` (struct :`G` 1.0 :`B` 0.068355 :`A` 1.0))
  (return _returnvalue _impactpoint))

(fn `spawn_decal_tracer`
  (params (Vocation :type "Vector Structure") (`spawn trnsofrm` :type "Vector Structure") (`Impact point` :type "Vector Structure"))
  (`|SpawnActorFromClass` "/Game/4/Bullet_decal.Bullet_decal_C" (`KismetMathLibrary.MakeTransform` `spawn trnsofrm` (`KismetMathLibrary.Conv_VectorToRotator` `Impact point`) (0.01 0.01 0.01)) "Undefined" "OverrideRootScale" null null)
  (if (>= (`KismetMathLibrary.RandomIntegerInRange` 1 10) 0)
    (`|SpawnActorFromClass` "/Game/4/Tracer_BP.Tracer_BP_C" (`KismetMathLibrary.MakeTransform` Vocation (`SceneComponent.K2_GetComponentRotation` (`/Game/FirstPersonBP/Blueprints/FirstPersonCharacter.FirstPersonCamera` (cast `/Game/FirstPersonBP/Blueprints/FirstPersonCharacter` (`GameplayStatics.GetPlayerCharacter` 0) :!pure true))) (0.1 0.1 0.1)) "Undefined" "OverrideRootScale" null null))
  (return))

(fn `UserConstructionScript`
  (`parent.UserConstructionScript`)
  (set `self.Max_Ammo` 20)
  (set `self.Ammo_Count` 20)
  (set `self.Reloading_Time` 2.0)
  (set `self.Bullet_Sprey` 200.0)
  (set `self.Name` "NewEnumerator3")
  (set `self.Variable_mode` false))