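; AWP sniper rifle weapon for the first-person character, with firing, reload, scope and unequip.
; Fire runs a camera line trace with random spread, spawns a decal and tracer, and plays sound, animations and muzzle flash, without applying damage.
; Scope shows an overlay widget, hides the arms and weapon, and uses timelines to blend FOV and arm position.
; Unequip saves ammo and weapon stats to the character's primary slot.
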(event `self.Unequip`
  (set `/Game/FirstPersonBP/Blueprints/FirstPersonCharacter.Primari_AK` (make `/Game/Blueprints/gun_data` "AWP_Weapon_C" "NewEnumerator4" (`self.Ammo_Count`) (`self.Max_Ammo`) (`self.Reloading_Time`) (`self.Bullet_Sprey`)) (cast `/Game/FirstPersonBP/Blueprints/FirstPersonCharacter` (`GameplayStatics.GetPlayerCharacter` 0) :!pure true)))

(event `self.Fire`
  (if (`self.can_fire`)
    (set `self.can_fire` false)
    (if (> (`self.Ammo_Count`) 0)
      (`SceneComponent.K2_SetRelativeTransform` (`/Game/FirstPersonBP/Blueprints/FirstPersonCharacter.Mesh2P` (cast `/Game/FirstPersonBP/Blueprints/FirstPersonCharacter` (`GameplayStatics.GetPlayerCharacter` 0) :!pure true)) (`KismetMathLibrary.MakeTransform` (5.898139 -6.467392 -25.529276)) false false)
      (`self.Ammo_check`)
      (bind (_start_location _impactpoint) (`self.Line_Trace`))
      (`self.spawn_decal_tracer` _start_location _impactpoint _impactpoint)
      (`|PlayMontage` (`/Game/FirstPersonBP/Blueprints/FirstPersonCharacter.Mesh2P` (cast `/Game/FirstPersonBP/Blueprints/FirstPersonCharacter` (`GameplayStatics.GetPlayerCharacter` 0) :!pure true)) "/Game/9/Arms_AWP_Fire_anim_Montage.Arms_AWP_Fire_anim_Montage"
        (:`then`
          (`self.Flash`)
          (`KismetSystemLibrary.Delay` 1.0)
          (set `self.can_fire` true)))
      (else
        (`GameplayStatics.PlaySound2D` "/Game/4/DryFire.DryFire" 1.0 1.0 0.0 null null)))))

(event `self.Reload`
  (bind _asfirst_person_character (cast `/Game/FirstPersonBP/Blueprints/FirstPersonCharacter` (`GameplayStatics.GetPlayerCharacter` 0) :!pure true))
  (if (< (`self.Ammo_Count`) (`self.Max_Ammo`))
    (`/Engine/EditorBlueprintResources/StandardMacros.DoOnce` false :!label _label
      (:`Completed`
        (set `/Game/FirstPersonBP/Blueprints/FirstPersonCharacter.Is_reload` true _asfirst_person_character)
        (`|PlayMontage` (`/Game/FirstPersonBP/Blueprints/FirstPersonCharacter.Mesh2P` _asfirst_person_character) "/Game/2/Arms_Reload.Arms_Reload"
          (:`then`
            (`SkeletalMeshComponent.PlayAnimation` (`self.SkeletalMesh`) "/Game/2/AK_Reload_anim.AK_Reload_anim" false)
            (`KismetSystemLibrary.Delay` (`self.Reloading_Time`))
            (set `self.Ammo_Count` (`self.Max_Ammo`))
            (set `/Game/FirstPersonBP/Blueprints/FirstPersonCharacter.Is_reload` false (cast `/Game/FirstPersonBP/Blueprints/FirstPersonCharacter` (`GameplayStatics.GetPlayerCharacter` 0) :!pure true))
            (goto _label :!via `Reset`)))))))

(event `self.Scope`
  (params (Tog :type Boolean))
  (bind _asfirst_person_character (cast `/Game/FirstPersonBP/Blueprints/FirstPersonCharacter` (`GameplayStatics.GetPlayerCharacter` 0) :!pure true))
  (bind _firstpersoncamera (`/Game/FirstPersonBP/Blueprints/FirstPersonCharacter.FirstPersonCamera` _asfirst_person_character))
  (bind _mesh2p (`/Game/FirstPersonBP/Blueprints/FirstPersonCharacter.Mesh2P` _asfirst_person_character))
  (if Tog
    (bind _returnvalue (`|CreateWidget` "/Game/Blueprints/AWP_Widget.AWP_Widget_C"))
    (bind _output_get (set `self.AWP_Widget` _returnvalue))
    (`UserWidget.AddToViewport` _output_get 0)
    (`SceneComponent.SetVisibility` (`/Game/FirstPersonBP/Blueprints/FirstPersonCharacter.ChildActor` _asfirst_person_character) false false)
    (`SceneComponent.SetVisibility` _mesh2p false false)
    (bind (_direction _newtrack_0) (`Timeline|Timeline_0` :!via `PlayFromStart`)
      (:`Update`
        (`CameraComponent.SetFieldOfView` _firstpersoncamera (`KismetMathLibrary.Lerp` 90.0 (`self.scope_X`) _newtrack_0))
        (`SceneComponent.K2_SetRelativeTransform` _mesh2p (`KismetMathLibrary.MakeTransform` (`KismetMathLibrary.VLerp` (5.898139 -6.467392 -25.529276) (5.898139 0.0 -16.0) _newtrack_0)) false false)
        (`Widget.SetVisibility` (`self.AWP_Widget`) "Visible")))
    (else
      (`Widget.SetVisibility` (`self.AWP_Widget`) "Hidden")
      (`SceneComponent.SetVisibility` (`/Game/FirstPersonBP/Blueprints/FirstPersonCharacter.ChildActor` (cast `/Game/FirstPersonBP/Blueprints/FirstPersonCharacter` (`GameplayStatics.GetPlayerCharacter` 0) :!pure true)) true false)
      (`SceneComponent.SetVisibility` (`/Game/FirstPersonBP/Blueprints/FirstPersonCharacter.Mesh2P` (cast `/Game/FirstPersonBP/Blueprints/FirstPersonCharacter` (`GameplayStatics.GetPlayerCharacter` 0) :!pure true)) true false)
      (bind (_direction_2 _newtrack_0_2) (`Timeline|Timeline_1` :!via `PlayFromStart`)
        (:`Update`
          (`CameraComponent.SetFieldOfView` _firstpersoncamera (`KismetMathLibrary.Lerp` (`self.scope_X`) 90.0 _newtrack_0_2))
          (`SceneComponent.K2_SetRelativeTransform` _mesh2p (`KismetMathLibrary.MakeTransform` (`KismetMathLibrary.VLerp` (5.898139 0.0 -16.0) (5.898139 -6.467392 -25.529276) _newtrack_0_2)) false false))))))

(event `self.ReceiveBeginPlay`
  (bind _returnvalue (`|CreateWidget` "/Game/Blueprints/AWP_Widget.AWP_Widget_C"))
  (set `self.AWP_Widget` _returnvalue))

(fn `Ammo_check`
  (bind _returnvalue (`KismetMathLibrary.RandomFloatInRange` 0.7 1.2))
  (`/Engine/EditorBlueprintResources/StandardMacros.DecrementInt` (`self.Ammo_Count`)
    (:`  `
      (`GameplayStatics.PlaySoundAtLocation` "/Game/4/Gunshot.Gunshot" (`self.K2_GetActorLocation`) (struct) (* _returnvalue 2.5) _returnvalue 0.0 "/Game/4/NewSoundAttenuation.NewSoundAttenuation" "/Game/4/NewSoundConcurrency.NewSoundConcurrency" null)
      (`SkeletalMeshComponent.PlayAnimation` (`self.SkeletalMesh`) "/Game/2/AK_Fire_anim.AK_Fire_anim" false))))

(fn `Line_Trace`
  (returns (`Start location` :type "Vector Structure") (ImpactPoint :type "Vector Structure"))
  (bind _bullet_sprey (`self.Bullet_Sprey`))
  (bind _returnvalue (`SceneComponent.K2_GetComponentLocation` (`self.Scene`)))
  (bind _returnvalue_2 (* _bullet_sprey -1.0))
  (bind _firstpersoncamera (`/Game/FirstPersonBP/Blueprints/FirstPersonCharacter.FirstPersonCamera` (cast `/Game/FirstPersonBP/Blueprints/FirstPersonCharacter` (`GameplayStatics.GetPlayerCharacter` 0) :!pure true)))
  (bind _returnvalue_3 (`SceneComponent.K2_GetComponentLocation` _firstpersoncamera))
  (bind _outhit (`KismetSystemLibrary.LineTraceSingle` _returnvalue_3 (+ (+ _returnvalue_3 (* (`SceneComponent.GetForwardVector` _firstpersoncamera) 20000.0)) (`KismetMathLibrary.MakeVector` (`KismetMathLibrary.RandomFloatInRange` _returnvalue_2 _bullet_sprey) (`KismetMathLibrary.RandomFloatInRange` _returnvalue_2 _bullet_sprey) (`KismetMathLibrary.RandomFloatInRange` _returnvalue_2 _bullet_sprey))) "TraceTypeQuery1"))
  (bind (_bblockinghit _binitialoverlap _time _distance _location _impactpoint) (`GameplayStatics.BreakHitResult` _outhit))
  (`KismetSystemLibrary.LineTraceSingle` :`Start` _returnvalue :`End` _impactpoint :`TraceChannel` "TraceTypeQuery1" :`TraceColor` (struct :`G` 1.0 :`B` 0.068355 :`A` 1.0))
  (return _returnvalue _impactpoint))

(fn `spawn_decal_tracer`
  (params (Vocation :type "Vector Structure") (`spawn trnsofrm` :type "Vector Structure") (`Impact point` :type "Vector Structure"))
  (`|SpawnActorFromClass` "/Game/4/Bullet_decal.Bullet_decal_C" (`KismetMathLibrary.MakeTransform` `spawn trnsofrm` (`KismetMathLibrary.Conv_VectorToRotator` `Impact point`) (0.01 0.01 0.01)) "Undefined" "OverrideRootScale" null null)
  (if (>= (`KismetMathLibrary.RandomIntegerInRange` 1 10) 0)
    (`|SpawnActorFromClass` "/Game/4/Tracer_BP.Tracer_BP_C" (`KismetMathLibrary.MakeTransform` Vocation (`SceneComponent.K2_GetComponentRotation` (`/Game/FirstPersonBP/Blueprints/FirstPersonCharacter.FirstPersonCamera` (cast `/Game/FirstPersonBP/Blueprints/FirstPersonCharacter` (`GameplayStatics.GetPlayerCharacter` 0) :!pure true))) (0.1 0.1 0.1)) "Undefined" "OverrideRootScale" null null))
  (return))

(fn `UserConstructionScript`
  (`parent.UserConstructionScript`)
  (set `self.Max_Ammo` 10)
  (set `self.Ammo_Count` 10)
  (set `self.Reloading_Time` 2.0)
  (set `self.Bullet_Sprey` 1.0)
  (set `self.Name` "NewEnumerator4")
  (set `self.Variable_mode` false))